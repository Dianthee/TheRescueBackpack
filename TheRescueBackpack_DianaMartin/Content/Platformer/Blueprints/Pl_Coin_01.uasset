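; Platformer coin pickup actor that plays a collection effect when an actor tagged "player" overlaps it.
; On overlap it activates its particle system, speeds up its rotating movement and starts a timeline that lifts it from its spawn point while shrinking the mesh.
; When the timeline finishes, it spawns a confetti burst at the mesh and destroys itself; no score or count is updated here.
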(event EventBeginPlay
  (Variables|Default|SetCoinInitPossition (Transformation|GetActorLocation))
  (Variables|Default|SetCoinEndPossition (+ (Variables|Default|GetCoinInitPossition) "0, 0,300.000000")))

(event Collision|EventActorBeginOverlap
  (params (OtherActor :type Actor%20Object%20Reference))
  (if (Actor|ActorHasTag OtherActor "player")
    (Components|Activation|Activate (Variables|Default|GetParticleSystem) false)
    (Variables|/Script/Engine.RotatingMovementComponent|SetRotationRate (Variables|Default|GetRotatingMovement) "0,1080.000000, 0")
    (bind _elevation_track (Timeline|Timeline_0 PlayFromStart)
      (:Update
        (Transformation|SetActorLocation (Math|Vector|Lerp(Vector) (Variables|Default|GetCoinInitPossition) (Variables|Default|GetCoinEndPossition) _elevation_track) false false)
        (Transformation|SetWorldScale3D (Variables|Default|GetStaticMesh) (- "1.000000,1.000000,1.000000" (* _elevation_track 0.5))))
      (:Finished
        (Effects|SpawnEmitteratLocation "/Game/Particles/Confetti_Particle.Confetti_Particle" (Transformation|GetWorldLocation (Variables|Default|GetStaticMesh)) "0, 0, 0" "0.300000,0.300000,0.300000")
        (Components|Activation|Deactivate (Variables|Default|GetParticleSystem))
        (Actor|DestroyActor)))))

(fn ConstructionScript)