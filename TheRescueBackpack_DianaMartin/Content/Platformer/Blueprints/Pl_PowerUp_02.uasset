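; Platformer power-up actor that animates its static mesh by moving an emissive highlight through its material slots; no pickup logic is present.
; BeginPlay lights the slot at Count and starts a looping timer on TimeToChange.
; Each tick of the timer restores that slot's plastic material, steps Count down with wrap-around, then applies the emissive material to the new slot.
; Count indexes both material arrays and the mesh slot alike.
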(event Custom|LoopEmissive
  (Utilities|SetPlastic)
  (Utilities|SetCountMaterial
    (:%20%20
      (Utilities|SetEmissive))))

(event EventBeginPlay
  (Utilities|Time|SetTimerbyEvent (delegate Custom|LoopEmissive) (Variables|Default|GettimeToChange) true)
  (Utilities|SetEmissive))

(fn ConstructionScript)