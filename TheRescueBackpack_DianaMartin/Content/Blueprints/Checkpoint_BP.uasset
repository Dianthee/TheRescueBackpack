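; Checkpoint trigger that writes the player's progress to the "check" save slot when an actor tagged "player" overlaps its box.
; If its Load flag is set, it stores the third-person character's location and a true Load flag, reusing the existing save or creating one.
; Otherwise it only clears the Load flag in the existing save, leaving the stored location untouched.
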(event OnComponentBeginOverlap(Box)
  (params (OverlappedComponent :type Primitive%20Component%20Object%20Reference) (OtherActor :type Actor%20Object%20Reference) (OtherComp :type Primitive%20Component%20Object%20Reference) (OtherBodyIndex :type Integer) (bFromSweep :type Boolean) (SweepResult :type Hit%20Result%20Structure%20%28by%20ref%29))
  (if (Actor|ActorHasTag OtherActor "player")
    (if (Variables|Default|GetLoad?)
      (Utilities|FlowControl|Sequence
        (:then_0
          (bind _asthird_person_character (Utilities|Casting|CastToThirdPersonCharacter (Game|GetPlayerCharacter 0)))
          (Variables|Default|SetPlayer_Location (Transformation|GetActorLocation _asthird_person_character)))
        (:then_1
          (bind _returnvalue (SaveGame|DoesSaveGameExist "check"))
          (if _returnvalue
            (bind _returnvalue_2 (SaveGame|LoadGamefromSlot "check"))
            (bind _assave (Utilities|Casting|CastToSave _returnvalue_2))
            (Variables|/Game/Blueprints/Save.Save_C|SetPlayerLoc_S _assave (Variables|Default|GetPlayer_Location))
            (Variables|/Game/Blueprints/Save.Save_C|SetLoad? _assave true)
            (SaveGame|SaveGametoSlot _assave "check")
            (else
              (bind _returnvalue_3 (SaveGame|CreateSaveGameObject "/Game/Blueprints/Save.Save_C"))
              (Variables|/Game/Blueprints/Save.Save_C|SetPlayerLoc_S _returnvalue_3 (Variables|Default|GetPlayer_Location))
              (Variables|/Game/Blueprints/Save.Save_C|SetLoad? _returnvalue_3 true)
              (SaveGame|SaveGametoSlot _returnvalue_3 "check")))))
      (else
        (bind _returnvalue_4 (SaveGame|LoadGamefromSlot "check"))
        (bind _assave_2 (Utilities|Casting|CastToSave _returnvalue_4))
        (Variables|/Game/Blueprints/Save.Save_C|SetLoad? _assave_2 false)
        (SaveGame|SaveGametoSlot _assave_2 "check")))))

(fn ConstructionScript)