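; Skewers is a hazard actor with a moving group of spikes that kills the player on contact.
; On BeginPlay it caches the world locations of two marker spheres, then a timeline lerps the skewer group between them without sweeping.
; An overlap on the box with an actor tagged "player" casts it to Character_BP and calls Dead.
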(event OnComponentBeginOverlap(Box)
  (params (OverlappedComponent :type Primitive%20Component%20Object%20Reference) (OtherActor :type Actor%20Object%20Reference) (OtherComp :type Primitive%20Component%20Object%20Reference) (OtherBodyIndex :type Integer) (bFromSweep :type Boolean) (SweepResult :type Hit%20Result%20Structure%20%28by%20ref%29))
  (if (Actor|ActorHasTag OtherActor "player")
    (bind _ascharacter_bp (Utilities|Casting|CastToCharacter_BP OtherActor))
    (Default|Dead _ascharacter_bp)))

(event EventBeginPlay
  (Variables|Default|SetposInitial (Transformation|GetWorldLocation (Variables|Default|GetSpherePosInitial)))
  (Variables|Default|SetposFinal (Transformation|GetWorldLocation (Variables|Default|GetSpherePosFinal)))
  (bind _position (Timeline|Timeline_0 Play)
    (:Update
      (Transformation|SetWorldLocation (Variables|Default|GetSkewers_Group) (Math|Vector|Lerp(Vector) (Variables|Default|GetposInitial) (Variables|Default|GetposFinal) _position) false false))))

(fn ConstructionScript)