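; Skewer ball hazard Blueprint that kills the player character on contact.
; Box overlap with an actor tagged "player" casts it to Character_BP, calls Dead and prints a debug string.
; A Timeline lerp that would move SkewersGroup between two sphere marker positions is present but unconnected, so this Blueprint does not move the skewers.
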(event OnComponentBeginOverlap(Box)
  (params (OverlappedComponent :type Primitive%20Component%20Object%20Reference) (OtherActor :type Actor%20Object%20Reference) (OtherComp :type Primitive%20Component%20Object%20Reference) (OtherBodyIndex :type Integer) (bFromSweep :type Boolean) (SweepResult :type Hit%20Result%20Structure%20%28by%20ref%29))
  (if (Actor|ActorHasTag OtherActor "player")
    (bind _ascharacter_bp (Utilities|Casting|CastToCharacter_BP OtherActor))
    (Default|Dead _ascharacter_bp)
    (Development|PrintString "Hello")))

(event EventBeginPlay)

(fn ConstructionScript)